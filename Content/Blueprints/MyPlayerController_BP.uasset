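; Player controller Blueprint that shows a mouse-following tooltip describing the primitive under the cursor.
; On BeginPlay it creates a PrimitiveTooltip widget, adds it to the viewport collapsed, and Tick repositions it to the mouse position plus an offset.
; OnPrimitiveHovered passes the hovered primitive's characteristics to the widget and makes it visible, and OnPrimitiveLeave collapses it again.
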(event `self.ReceiveBeginPlay`
  (bind _returnvalue (`|CreateWidget` "/Game/Blueprints/UI/PrimitiveTooltip.PrimitiveTooltip_C"))
  (bind _output_get (set `self.PrimitiveTooltipWidgetRef` _returnvalue))
  (`Widget.SetVisibility` _output_get "Collapsed")
  (`UserWidget.AddToViewport` _output_get 0))

(event `self.ReceiveTick`
  (params (DeltaSeconds :type "Float (single-precision)"))
  (bind _primitivetooltipwidgetref (`self.PrimitiveTooltipWidgetRef`))
  (`/Engine/EditorBlueprintResources/StandardMacros.IsValid` _primitivetooltipwidgetref
    (:`Is Valid`
      (bind _returnvalue (`WidgetLayoutLibrary.GetMousePositionOnViewport`))
      (`UserWidget.SetPositionInViewport` _primitivetooltipwidgetref (+ _returnvalue (`self.TooltipOffset`)) false))))

(event `self.OnPrimitiveHovered`
  (params (HoveredPrimitive :type "PrimitiveBase Object Reference (by ref)"))
  (bind _primitivetooltipwidgetref (`self.PrimitiveTooltipWidgetRef`))
  (`/Engine/EditorBlueprintResources/StandardMacros.IsValid` _primitivetooltipwidgetref
    (:`Is Valid`
      (bind _returnvalue (`PrimitiveBase.GetPrimitiveCharacteristics` HoveredPrimitive))
      (`/Game/Blueprints/UI/PrimitiveTooltip.Event UpdateCharactesirtics` _primitivetooltipwidgetref _returnvalue)
      (`Widget.SetVisibility` _primitivetooltipwidgetref "Visible"))))

(event `self.OnPrimitiveLeave`
  (bind _primitivetooltipwidgetref (`self.PrimitiveTooltipWidgetRef`))
  (`/Engine/EditorBlueprintResources/StandardMacros.IsValid` _primitivetooltipwidgetref
    (:`Is Valid`
      (if (`Widget.IsInViewport` _primitivetooltipwidgetref)
        (`Widget.SetVisibility` (`self.PrimitiveTooltipWidgetRef`) "Collapsed")))))

(fn `UserConstructionScript`)